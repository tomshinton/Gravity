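; BP_PolyFinder is a gravity prototype actor that probes surrounding geometry and visualizes how strongly it would pull, using debug lines only.
; Its FindPoly event clears old lines, then sweeps one-degree Visibility line traces around a full circle in a fixed plane, out to InfluenceCutoff.
; Each hit draws a red line whose thickness follows a clamped inverse of distance scaled by GravityFalloff; no force is applied.
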(event Custom|FindPoly
  (bind _returnvalue (Transformation|GetActorLocation))
  (Rendering|Debug|FlushPersistentDebugLines)
  (for _index (range 0 359)
    (bind (_outhit _returnvalue_2) (Collision|LineTraceByChannel _returnvalue (+ _returnvalue (* (Math|Vector|GetForwardVector (Math|Rotator|CombineRotators (Math|Rotator|MakeRotator 0.0 (Math|Conversions|ToFloat(Integer) _index) 0.0) "0,90.000000, 0")) (Math|Conversions|ToVector(Float) (Variables|Default|GetInfluenceCutoff)))) "TraceTypeQuery1" false 0 "None"))
    (if _returnvalue_2
      (Rendering|Debug|DrawDebugLine (.TraceStart (Collision|BreakHitResult _outhit)) (.ImpactPoint (Collision|BreakHitResult _outhit)) "(R=0.390625,G=0.000000,B=0.000000,A=1.000000)" 1e+02 (* 5e+02 (Math|Float|Clamp(Float) (/ 1.0 (* (.Distance (Collision|BreakHitResult _outhit)) (Variables|Default|GetGravityFalloff)))))))))

(event EventBeginPlay)

(event Collision|EventActorBeginOverlap
  (params (OtherActor :type Actor%20Object%20Reference)))

(event EventTick
  (params (DeltaSeconds :type Float%20%28single-precision%29)))

(fn ConstructionScript)